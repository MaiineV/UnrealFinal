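; Lever Blueprint that opens a door once when its Pull event fires, using the IsOpen flag to ignore later pulls.
; A MoveTimeLine curve drives world rotation of both Door and Lever, each toward a 90-degree offset on different axes.
; Each update lerps from the current rotation rather than a cached start, so the rotation compounds over the timeline.
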(event Custom|Pull
  (bind _door (Variables|Default|GetDoor))
  (bind _lever (Variables|Default|GetLever))
  (bind _returnvalue (Transformation|GetWorldRotation _door))
  (bind _returnvalue_2 (Transformation|GetWorldRotation _lever))
  (if (not (Variables|Default|GetIsOpen))
    (Variables|Default|SetIsOpen true)
    (bind _movey (Timeline|MoveTimeLine Play)
      (:Update
        (Transformation|SetWorldRotation (Variables|Default|GetDoor) (Math|Rotator|Lerp(Rotator) _returnvalue (Math|Rotator|CombineRotators _returnvalue "0,90.000000, 0") _movey) false false)
        (Transformation|SetWorldRotation (Variables|Default|GetLever) (Math|Rotator|Lerp(Rotator) _returnvalue_2 (Math|Rotator|CombineRotators _returnvalue_2 "-90.000000,0.000000, 0") _movey) false false)))))

(fn ConstructionScript)